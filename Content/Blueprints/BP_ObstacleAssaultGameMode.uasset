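; Game mode for the Obstacle Assault game that handles player falls, lives and game over.
; On BeginPlay it saves the player pawn's location as the respawn point and hands the pawn to FallDetector for tracking.
; Tick polls the detector, costing a life on a fall and moving the pawn back to the saved location.
; When lives run out, it prints "Game Over", sets the game-over flag and destroys the pawn.
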(event `self.ReceiveBeginPlay`
  (`self.StorePlayerLocation`)
  (`FallDetectorComponent.SetTrackedActor` (`self.FallDetector`) (`GameplayStatics.GetPlayerPawn` 0)))

(event `self.ReceiveTick`
  (params (DeltaSeconds :type "Float (single-precision)"))
  (if (`self.IsGameOver`)
    _
    (elif (`FallDetectorComponent.HasFell` (`self.FallDetector`))
      (bind _output_get (set `self.PlayerLivesCount` (- (`self.PlayerLivesCount`) 1)))
      (if (<= _output_get 0)
        (`KismetSystemLibrary.PrintString` "Game Over")
        (set `self.IsGameOver` true)
        (`self.K2_DestroyActor` (`GameplayStatics.GetPlayerPawn` 0))
        (else
          (`self.ResetPlayerLocation`))))))

(fn `ResetPlayerLocation`
  (`self.K2_SetActorLocation` (`GameplayStatics.GetPlayerPawn` 0) (`self.PlayerSavedLocation`) false false)
  (return))

(fn `StorePlayerLocation`
  (set `self.PlayerSavedLocation` (`self.K2_GetActorLocation` (`GameplayStatics.GetPlayerPawn` 0)))
  (return))

(fn `UserConstructionScript`)