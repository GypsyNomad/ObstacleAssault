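; Game mode for an obstacle course that manages lives, checkpoint respawns, game over and finish timing.
; Tick polls a FallDetector tracking the player; each fall costs a life and either teleports the pawn to the saved location or detaches the camera and restarts the level after a delay.
; Checkpoint events update the respawn point, and finishing shows formatted elapsed time from server world time.
; Widgets display welcome, lives, checkpoint and end screens.
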(event `self.ReceiveBeginPlay`
  (`self.StorePlayerLocation`)
  (`FallDetectorComponent.SetTrackedActor` (`self.FallDetector`) (`GameplayStatics.GetPlayerPawn` 0))
  (set `self.IsGameOver` false)
  (bind _returnvalue (`|CreateWidget` "/Game/Blueprints/Widgets/WBP_Welcome.WBP_Welcome_C"))
  (`UserWidget.AddToViewport` _returnvalue 0)
  (bind _returnvalue_2 (`|CreateWidget` "/Game/Blueprints/Widgets/WBP_LivesCounter.WBP_LivesCounter_C"))
  (bind _output_get (set `self.LivesCounterWidget` _returnvalue_2))
  (`UserWidget.AddToViewport` _output_get 0)
  (`self.SetLivesCountText`)
  (`self.StoreLevelStartTime`))

(event `self.ReceiveTick`
  (params (DeltaSeconds :type "Float (single-precision)"))
  (if (`self.IsGameOver`)
    _
    (elif (`FallDetectorComponent.HasFell` (`self.FallDetector`))
      (`self.Event_ActorFell`))))

(event `Event_ActorFell`
  (`self.ReduceLivesCount`)
  (`self.SetLivesCountText`)
  (if (<= (`self.PlayerLivesCount`) 0)
    (set `self.IsGameOver` true)
    (`self.DetachPlayerCamera`)
    (`GameplayStatics.PlaySound2D` "/Game/LearningKit_Games/Assets/SFX/SFX_Wind_Long.SFX_Wind_Long" 1.0 1.0 0.0 null null)
    (bind _returnvalue (`|CreateWidget` "/Game/Blueprints/Widgets/WBP_GameOver.WBP_GameOver_C"))
    (`UserWidget.AddToViewport` _returnvalue 0)
    (`KismetSystemLibrary.Delay` 10.0)
    (`self.RestartLevel`)
    (else
      (`self.ResetPlayerLocation`)
      (`GameplayStatics.PlaySound2D` "/Game/LearningKit_Games/Assets/SFX/SFX_Wind_Short.SFX_Wind_Short" 1.0 1.0 0.0 null null))))

(event `Event_CheckpointReached`
  (params (Checkpoint :type "Actor Object Reference"))
  (set `self.PlayerSavedLocation` (`self.K2_GetActorLocation` Checkpoint))
  (bind _returnvalue (`|CreateWidget` "/Game/Blueprints/Widgets/WBP_Checkpoint.WBP_Checkpoint_C"))
  (`UserWidget.AddToViewport` _returnvalue 0))

(event `Event_SuccessfulFinish`
  (`GameplayStatics.PlaySound2D` "/Game/LearningKit_Robots/Audio/Success_V2.Success_V2" 1.0 1.0 0.0 null null)
  (bind _returnvalue (`|CreateWidget` "/Game/Blueprints/Widgets/WBP_SuccessFinish.WBP_SuccessFinish_C"))
  (`UserWidget.AddToViewport` _returnvalue 0)
  (bind _elapsed (`self.GetElapsedTime`))
  (bind _formattedtime (`self.FormatTime` _elapsed))
  (`TextBlock.SetText` (`/Game/Blueprints/Widgets/WBP_SuccessFinish.TimeToCompleteText` _returnvalue) _formattedtime))

(fn `DestroyPlayerPawn`
  (set `self.IsGameOver` true)
  (`self.K2_DestroyActor` (`GameplayStatics.GetPlayerPawn` 0))
  (return))

(fn `DetachPlayerCamera`
  (bind _asbp_player (cast `/Game/Blueprints/Characters/BP_Player` (`GameplayStatics.GetPlayerPawn` 0)))
  (`/Game/Blueprints/Characters/BP_Player.Event_PlayerLost` _asbp_player)
  (return))

(fn `FormatTime`
  (params (Time :type "Float (double-precision)"))
  (returns (FormattedTime :type Text))
  (bind _returnvalue (`KismetMathLibrary.FTrunc` Time))
  (return (`|FormatText` "{0}:{1}.{2}" (`KismetTextLibrary.Conv_IntToText` (/ (mod _returnvalue 3600) 60) false true 2) (`KismetTextLibrary.Conv_IntToText` (mod _returnvalue 60) false true 2) (`KismetTextLibrary.Conv_IntToText` (`KismetMathLibrary.FTrunc` (* (- Time _returnvalue) 1000.0)) false true 3))))

(fn `GetElapsedTime`
  (returns (Elapsed :type "Float (double-precision)"))
  (return (- (`GameStateBase.GetServerWorldTimeSeconds` (`GameplayStatics.GetGameState`)) (`self.LevelTimer`))))

(fn `ReduceLivesCount`
  (set `self.PlayerLivesCount` (- (`self.PlayerLivesCount`) 1))
  (return))

(fn `ResetPlayerLocation`
  (`self.K2_SetActorLocation` (`GameplayStatics.GetPlayerPawn` 0) (`self.PlayerSavedLocation`) false false)
  (return))

(fn `RestartLevel`
  (bind _returnvalue (`GameplayStatics.GetCurrentLevelName` true))
  (`GameplayStatics.OpenLevel` (`KismetStringLibrary.Conv_StringToName` _returnvalue)))

(fn `SetLivesCountText`
  (`TextBlock.SetText` (`/Game/Blueprints/Widgets/WBP_LivesCounter.LivesCounter` (`self.LivesCounterWidget`)) (`|FormatText` "Lives: {0}" (`KismetTextLibrary.Conv_IntToText` (`self.PlayerLivesCount`))))
  (return))

(fn `StoreLevelStartTime`
  (set `self.LevelTimer` (`GameStateBase.GetServerWorldTimeSeconds` (`GameplayStatics.GetGameState`)))
  (return))

(fn `StorePlayerLocation`
  (set `self.PlayerSavedLocation` (`self.K2_GetActorLocation` (`GameplayStatics.GetPlayerPawn` 0)))
  (return))

(fn `UserConstructionScript`)